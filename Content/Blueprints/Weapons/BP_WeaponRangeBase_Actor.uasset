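; BP_WeaponRangeBase_Actor is a base actor for ranged weapons, storing the owning character passed in through InitializeWeapon.
; GetOwnerRotation returns the owner's control rotation, falling back to actor rotation when their yaw differs by over 45 degrees.
; GetMuzzlePosition reads a named socket on the skeletal mesh.
; Fire and reload events are empty here, and a visibility line trace sits unconnected.
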(event Custom|Fire_Event)

(event Custom|Reload_Event)

(event Custom|InitializeWeapon
  (params (CharacterOwner :type BP%20Third%20Person%20Character%20Object%20Reference))
  (Variables|Owner|SetCharacterOwner CharacterOwner))

(event EventBeginPlay)

(event Collision|EventActorBeginOverlap
  (params (OtherActor :type Actor%20Object%20Reference)))

(event EventTick
  (params (DeltaSeconds :type Float%20%28single-precision%29)))

(fn ConstructionScript)

(fn GetOwnerRotation
  (bind _characterowner (Variables|Owner|GetCharacterOwner))
  (bind _returnvalue (Pawn|GetControlRotation _characterowner :!class /Script/Engine.Pawn))
  (bind _returnvalue_2 (Transformation|GetActorRotation _characterowner))
  (return (select (> (Math|Float|Absolute(Float) (.yaw (Math|Rotator|Delta(Rotator) _returnvalue _returnvalue_2))) 45.0) _returnvalue_2 _returnvalue)))

(fn GetMuzzlePosition
  (return (Transformation|GetSocketLocation (Variables|Default|GetSkeletalMesh) (Variables|Settings|GetMuzzleSocketName))))